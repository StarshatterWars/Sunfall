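; Player hoverboard pawn for a race, with input held off until the controller's RaceStart flag is set.
; Five hover components act on a physics cube, driven by camera-forward force and yaw torque that inverts when moving backward.
; Drift notifies the HoverboardController and adds movement input.
; If flipped and slow across a three-second delay, the pawn is destroyed and the controller respawns the player, using the stored start transform.
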(event `self.ReceiveBeginPlay`
  (bind _board_sample_cube1 (`self.board_sample_Cube1`))
  ;[1 1 1] Event Begin Play. Controller Ref and Hover Components
  (`|ExecutionSequence`
    (:`then_0`
      (bind _ashoverboard_controller (cast `/Game/Blueprints/HoverboardController` (`GameplayStatics.GetPlayerController` 0)))
      (bind _output_get (set `self.ControllerRef` _ashoverboard_controller))
      (set `/Game/Blueprints/HoverboardController.RespawnLocation` (`self.GetTransform`) _output_get)
      (`self.DisableInput` (`self.ControllerRef`))
      (`PrimitiveComponent.SetCollisionEnabled` (`self.board_sample_Cube1`) "QueryAndPhysics"))
    (:`then_1`
      (`/Game/HoverComponent2.IntComponents` (`self.HoverComponent2`) _board_sample_cube1)
      (`/Game/HoverComponent2.IntComponents` (`self.HoverComponent3`) _board_sample_cube1)
      (`/Game/HoverComponent2.IntComponents` (`self.HoverComponent4`) _board_sample_cube1)
      (`/Game/HoverComponent2.IntComponents` (`self.HoverComponent5`) _board_sample_cube1)
      (`/Game/HoverComponent2.IntComponents` (`self.HoverComponent6`) _board_sample_cube1))))

(event `Key|Left`
  (params (Key :type "Key Structure"))
  (:`Pressed`
    (set `self.ForwardForce` 2500000.0))
  (:`Released`
    (set `self.ForwardForce` 7500000.0)
    (set `self.ForwardForce` 1000000.0)
    (set `self.DesiredRotate` (`KismetMathLibrary.ComposeRotators` (`self.DesiredRotate`)))))

(event `InputAxis|MoveForward`
  (params (AxisValue :type "Float (single-precision)"))
  ;[1 1 1] Moving Forward
  (`PrimitiveComponent.AddForce` (`self.board_sample_Cube1`) (* (* (`SceneComponent.GetForwardVector` (`self.Camera`)) 750000.0) AxisValue) "None" false))

(event `InputAction|Drift`
  (params (Key :type "Key Structure"))
  (:`Pressed`
    (`/Game/Blueprints/HoverboardController.Turning` (`self.ControllerRef`))
    (`self.AddMovementInput` (`KismetMathLibrary.MakeVector` 0.0 0.0 (* (`KismetMathLibrary.SelectFloat` 1.0 -1.0 (> (`KismetMathLibrary.Dot_VectorVector` (stale `InputAxis|MoveRight` _returnvalue) (`SceneComponent.GetForwardVector` (`self.Camera`))) 0.0)) (* (stale `InputAxis|MoveRight` AxisValue) 400000000.0))) (`self.DriftValue`))))

(event `Key|Right`
  (params (Key :type "Key Structure"))
  (:`Pressed`
    (set `self.ForwardForce` 7500000.0)
    (set `self.ForwardForce` 1000000.0)
    (set `self.DesiredRotate` (`KismetMathLibrary.ComposeRotators` (`self.DesiredRotate`))))
  (:`Released`
    (set `self.ForwardForce` 2500000.0)))

(event `InputAxis|MoveRight`
  (params (AxisValue :type "Float (single-precision)"))
  (bind _board_sample_cube1 (`self.board_sample_Cube1`))
  ;[1 1 1] Turning the Player
  (bind _returnvalue (`PrimitiveComponent.GetPhysicsLinearVelocity` _board_sample_cube1 "None"))
  (`PrimitiveComponent.AddTorqueInDegrees` _board_sample_cube1 (`KismetMathLibrary.MakeVector` 0.0 0.0 (* (`KismetMathLibrary.SelectFloat` 1.0 -1.0 (> (`KismetMathLibrary.Dot_VectorVector` _returnvalue (`SceneComponent.GetForwardVector` (`self.Camera`))) 0.0)) (* AxisValue 400000000.0))) "None" false))

(event `self.ReceiveTick`
  (params (DeltaSeconds :type "Float (single-precision)"))
  (bind _controllerref (`self.ControllerRef`))
  (bind _controllerref_2 (`self.ControllerRef`))
  ;[1 1 1] Event Tick, starts the race countdown.
  (if (`self.IsLocallyControlled`)
    (if (`/Game/Blueprints/HoverboardController.RaceStart` _controllerref)
      (`self.EnableInput` _controllerref)
      (`|ExecutionSequence`
        (:`then_1`
          ;[1 1 1] Respawns player when he fips over
          (bind _playerisstuck (`self.RespawnCheck`))
          (if _playerisstuck
            (`KismetSystemLibrary.Delay` 3.0)
            (bind _playerisstuck_2 (`self.RespawnCheck`))
            (if _playerisstuck_2
              (`self.K2_SetActorTransform` _controllerref_2 (`/Game/Blueprints/HoverboardController.RespawnLocation` _controllerref_2) false true)
              (`self.K2_DestroyActor` (`GameplayStatics.GetPlayerPawn` 0)))))))))

(event `self.ReceiveDestroyed`
  ;[1 1 1] Respawns player when he fips over
  (`/Game/Blueprints/HoverboardController.RespawnPlayer` (`self.ControllerRef`)))

(fn `Drift Function`)

(fn `RespawnCheck`
  (returns (PlayerIsStuck :type Boolean))
  (if (and (< (`KismetMathLibrary.Dot_VectorVector` (`self.GetActorUpVector`) (0.0 0.0 1.0)) 0.5) (< (`WheeledVehicleMovementComponent.GetForwardSpeed` (`self.VehcileMovement`)) 0.5))
    (set `self.Stuck?` true)
    (else
      (set `self.Stuck?` false)))
  (return (`self.Stuck?`)))

(fn `UserConstructionScript`)