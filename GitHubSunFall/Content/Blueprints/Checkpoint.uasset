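; Checkpoint actor for a hoverboard game that reports when the player clears it in the intended direction.
; When an overlap with its trigger ends, it casts player pawn 0 to the hoverboard and dot-tests that pawn's forward vector against the Arrow component's direction.
; On a positive result it calls CheckpointCleared with its number, hides its trigger, particles and mesh, and turns off overlap events.
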(event `self.Trigger.OnComponentEndOverlap`
  (params (OverlappedComponent :type "PrimitiveComponent Object Reference") (OtherActor :type "Actor Object Reference") (OtherComp :type "PrimitiveComponent Object Reference") (OtherBodyIndex :type Integer))
  (bind _trigger (`self.Trigger`))
  ;[1 1 1] Checkpoint System
  (bind _ashoverboard_bp1 (cast `/Game/HoverboardBP1` (`GameplayStatics.GetPlayerPawn` 0)))
  (if (> (`KismetMathLibrary.Dot_VectorVector` (`self.GetActorForwardVector` _ashoverboard_bp1) (`KismetMathLibrary.Conv_RotatorToVector` (`SceneComponent.K2_GetComponentRotation` (`self.Arrow`)))) 0.0)
    (`self.CheckpointCleared` (`self.CheckpointNumber`))
    (`SceneComponent.SetHiddenInGame` _trigger true false)
    (`SceneComponent.SetHiddenInGame` (`self.ParticleSystem`) true false)
    (`SceneComponent.SetHiddenInGame` (`self.StaticMesh`) true false)
    (set `PrimitiveComponent.bGenerateOverlapEvents` false _trigger)))

(fn `UserConstructionScript`)